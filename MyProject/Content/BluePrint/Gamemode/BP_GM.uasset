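; Game mode for a timed target game: the player wins when every BP_Sphere has died and loses when the countdown in Tick reaches zero.
; BeginPlay binds each sphere's OnDied to CountTarget and restores the remaining count from the GameInstance, defaulting to the sphere total.
; CountTarget writes each decrement back to the GameInstance.
; EndGame runs once, printing the result, playing UMG_MainUI's GameOver animation and passing the remaining time to BP_GI.SetBestTime.
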(event Custom|EndGame
  (params (IsVictory :type Boolean))
  ;[1 1 1] 한번 호출되면 막아버림
  (Utilities|FlowControl|DoOnce false
    (:Completed
      (if IsVictory
        (Development|PrintString "승리")
        (else
          (Development|PrintString "패배")))
      (bind _foundwidgets (Widget|GetAllWidgetsOfClass "/Game/BluePrint/UMG/UMG_MainUI.UMG_MainUI_C" true))
      (for _array_element _foundwidgets
        (Utilities|FlowControl|Sequence
          (:then_0
            (UserInterface|Animation|PlayAnimation _array_element (Variables|/Game/BluePrint/UMG/UMG_MainUI.UMG_MainUI_C|GetGameOver _array_element) 0.0 1 "Forward" 1.0 false)
            ;[1 1 1] Best Time 저장
            (bind _asbp_gi (Utilities|Casting|CastToBP_GI (Game|GetGameInstance)))
            (Default|SetBestTime _asbp_gi (Variables|Default|GetTime))))))))

(event Custom|OnEndPlay_이벤트
  (params (Actor :type Actor%20Object%20Reference) (EndPlayReason :type EEndPlayReason%20Enum :default "Destroyed"))
  ;[1 1 1] 이벤트 디스패처
  (CallFunction|CountTarget)
  (Game|UnbindEventfromOnEndPlay (delegate Custom|OnEndPlay_이벤트)))

(event Custom|OnDied_이벤트
  (CallFunction|CountTarget))

(event EventBeginPlay
  (Utilities|FlowControl|Sequence
    (:then_0
      (Variables|Default|SetTime (Variables|Default|GetMAXTime))
      (bind _outactors (Actor|GetAllActorsOfClass "/Game/BluePrint/BP_Sphere.BP_Sphere_C"))
      (Variables|Default|SetMAXTarget (Utilities|Array|Length _outactors))
      (for _array_element _outactors
        (EventDispatchers|AssignOnDied _array_element (delegate Custom|OnDied_이벤트))))
    (:then_1
      (bind _value (Class|IFGI|GetCount(Message) (Game|GetGameInstance)))
      (if (== _value 0)
        (Variables|Default|SetTargetCount (Variables|Default|GetMAXTarget))
        (else
          (Variables|Default|SetTargetCount _value))))))

(event EventTick
  (params (DeltaSeconds :type Float%20%28single-precision%29))
  (bind _output_get (Variables|Default|SetTime (- (Variables|Default|GetTime) DeltaSeconds)))
  (if (<= _output_get 0.0)
    ;[1 1 1] 패배
    (CallFunction|Endgame false)))

(fn ConstructionScript)

(fn CountTarget
  (bind _result (Math|Integer|DecrementInt (Variables|Default|GetTargetCount))
    (:%20%20
      (bind _output_get (Variables|Default|SetTargetCount _result))
      (Class|IFGI|SetCount(Message) (Game|GetGameInstance) _output_get)
      (if (== _output_get 0)
        (CallFunction|Endgame true)))))

(fn GetCount
  (return 0))