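; BP_Pawn is a pawn Blueprint that deals damage to whatever the camera points at on a left mouse click.
; A debug key event runs a Visibility line trace forward from the player camera, drawing it for debugging, and applies damage to the hit actor.
; Disconnected nodes for destroying the actor and spawning an explosion never run, and the other events are empty.
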(event EventBeginPlay)

(event Collision|EventActorBeginOverlap
  (params (OtherActor :type Actor%20Object%20Reference)))

(event EventTick
  (params (DeltaSeconds :type Float%20%28single-precision%29)))

(event Input|MouseEvents|DebugKeyLeftMouseButton
  (params (Key :type Key%20Structure :default "None") (ActionValue :type Input%20Action%20Value%20Structure))
  (bind _returnvalue (Game|GetPlayerCameraManager 0))
  (bind _returnvalue_2 (Transformation|GetActorLocation _returnvalue))
  (:Pressed
    (bind (_outhit _returnvalue_3) (Collision|LineTraceByChannel _returnvalue_2 (+ _returnvalue_2 (* (Math|Vector|GetForwardVector (Transformation|GetActorRotation _returnvalue)) 1e+04)) "TraceTypeQuery1" false 0 "ForDuration" true "(R=0.984375,G=0.968750,B=1.000000,A=1.000000)" "(R=0.989583,G=1.000000,B=1.000000,A=1.000000)" 0.0))
    (if _returnvalue_3
      (Game|Damage|ApplyDamage (.HitActor (Collision|BreakHitResult _outhit)) 1.0 0 0))))

(fn ConstructionScript)