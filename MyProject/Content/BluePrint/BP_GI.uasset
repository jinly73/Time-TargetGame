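; BP_GI is a Game Instance that holds a persistent best time and a Count value for the game.
; On Init it loads the SG_Time save from its slot and caches the best time, falling back to a fresh save object.
; SetBestTime keeps only a larger value and writes it straight to the slot.
; Count has a simple setter and getter and is not saved.
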(event Custom|SetBestTime
  (params (A :type Float%20%28double-precision%29))
  (bind _as_sg_time (Variables|Default|GetAs%20SG%20Time))
  (if (> A (Variables|Default|GetBestTime))
    (bind _output_get (Variables|Default|SetBestTime A))
    (Variables|/Game/BluePrint/SaveGame/SG_Time.SG_Time_C|SetBestTime _as_sg_time _output_get)
    (SaveGame|SaveGametoSlot _as_sg_time (Variables|/Game/BluePrint/SaveGame/SG_Time.SG_Time_C|GetSlotName _as_sg_time) (Variables|/Game/BluePrint/SaveGame/SG_Time.SG_Time_C|GetUserIndex _as_sg_time))))

(event EventSetCount
  (params (Value :type Integer))
  (Variables|Default|SetCount Value))

(event EventInit
  (bind _returnvalue (SaveGame|CreateSaveGameObject "/Game/BluePrint/SaveGame/SG_Time.SG_Time_C"))
  (bind _returnvalue_2 (SaveGame|LoadGamefromSlot (Variables|/Game/BluePrint/SaveGame/SG_Time.SG_Time_C|GetSlotName _returnvalue) (Variables|/Game/BluePrint/SaveGame/SG_Time.SG_Time_C|GetUserIndex _returnvalue)))
  (bind _assg_time (Utilities|Casting|CastToSG_Time _returnvalue_2)
    (:then
      (bind _output_get (Variables|Default|SetAs%20SG%20Time _assg_time))
      (Variables|Default|SetBestTime (Variables|/Game/BluePrint/SaveGame/SG_Time.SG_Time_C|GetBestTime _output_get)))
    (:CastFailed
      (Variables|Default|SetAs%20SG%20Time _returnvalue))))

(fn GetCount
  (return (Variables|Default|GetCount)))